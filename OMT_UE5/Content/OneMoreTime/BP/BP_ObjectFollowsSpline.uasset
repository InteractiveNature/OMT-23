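; BP_ObjectFollowsSpline is an actor with a configurable static mesh, named for moving along a spline, though the graph holds no movement logic.
; The construction script applies the chosen mesh, and BeginPlay caches the first SplineToFollow actor found in the level.
; MoveObject plays a timeline at a rate derived from the completion time in seconds, but no timeline output or spline sampling is wired up.
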(event `Move Object`
  (`TimelineComponent.SetPlayRate` (`self.Move Object T`) (/ 1.0 (`self.Time to Complete (In Sec)`)))
  (`Timeline|Move Object T`))

(event `self.ReceiveBeginPlay`
  (bind _returnvalue (`GameplayStatics.GetActorOfClass` (`self.Spline to Follow`)))
  (set `self.Spline REF_1` _returnvalue))

(fn `UserConstructionScript`
  (`StaticMeshComponent.SetStaticMesh` (`self.StaticMesh`) (`self.Set Static Mesh`)))