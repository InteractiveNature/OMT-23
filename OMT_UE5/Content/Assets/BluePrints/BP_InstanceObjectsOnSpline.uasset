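; Construction-script Blueprint that places copies of a chosen mesh at even intervals along a spline.
; It divides the spline length by Offset, then adds an instance to one InstancedStaticMesh component at each step, using local-space positions.
; Instances keep default rotation and unit scale, as the random scale, random rotation and material override nodes are not wired in.
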(fn `UserConstructionScript`
  (locals (`Number of Instances` :type Integer :default 0))
  (bind _offset (`self.Offset`))
  (`StaticMeshComponent.SetStaticMesh` (`self.InstancedStaticMesh`) (`self.Placed Mesh`))
  (bind _output_get (set `local.Number of Instances` (`KismetMathLibrary.FFloor` (/ (`SplineComponent.GetSplineLength` (`self.Spline`)) _offset))))
  (for _index (range (+ _output_get 1))
    (`InstancedStaticMeshComponent.AddInstance` (`self.InstancedStaticMesh`) (`KismetMathLibrary.MakeTransform` (`SplineComponent.GetLocationAtDistanceAlongSpline` (`self.Spline`) (* _index _offset) "Local") (`KismetMathLibrary.MakeRotator` 0.0) (1.0 1.0 1.0)) false)))