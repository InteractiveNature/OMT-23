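; Construction-script actor that lays randomly chosen static meshes along a spline as deforming spline mesh components.
; Each segment spans SplineLength in distance, taking local positions and tangents from the spline, with tangents clamped to that length.
; The loop runs up to the floored total spline length, not divided by SplineLength; that division is left unconnected.
; Event graph stubs are empty.
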(fn `UserConstructionScript`
  (bind _spline (`self.Spline`))
  (for _index (range (+ (`KismetMathLibrary.FFloor` (`SplineComponent.GetSplineLength` (`self.Spline`))) 1))
    (bind _returnvalue (`AddComponent|NODE_AddSplineMeshComponent-0`))
    (`StaticMeshComponent.SetStaticMesh` _returnvalue (`KismetArrayLibrary.Array_Random` (`self.Meshes`)))
    (bind _returnvalue_2 (* _index (`self.Spline Length`)))
    (bind _returnvalue_3 (* (+ _index 1) (`self.Spline Length`)))
    (`SplineMeshComponent.SetStartAndEnd` _returnvalue (`SplineComponent.GetLocationAtDistanceAlongSpline` _spline _returnvalue_2 "Local") (`KismetMathLibrary.ClampVectorSize` (`SplineComponent.GetTangentAtDistanceAlongSpline` _spline _returnvalue_2 "Local") 0.0 (`self.Spline Length`)) (`SplineComponent.GetLocationAtDistanceAlongSpline` _spline _returnvalue_3 "Local") (`KismetMathLibrary.ClampVectorSize` (`SplineComponent.GetTangentAtDistanceAlongSpline` _spline _returnvalue_3 "Local") 0.0 (`self.Spline Length`)) true)))